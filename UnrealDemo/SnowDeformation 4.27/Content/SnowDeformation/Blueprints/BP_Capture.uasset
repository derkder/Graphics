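; Scene capture actor for the snow deformation system that publishes its capture area size to materials.
; On BeginPlay it writes the SceneCapture OrthoWidth to the CaptureSize parameter of MPC_Capture.
; DrawToPersistent, MoveCapture and Tick are empty stubs.
; SnapToPixelWorldSize holds only an unconnected math expression that would snap player XY to pixel-sized world steps with a half-pixel offset.
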(event EventBeginPlay
  (Rendering|Material|SetScalarParameterValue "/Game/SnowDeformation/Materials/MPC_Capture.MPC_Capture" "CaptureSize" (Variables|/Script/Engine.SceneCaptureComponent2D|GetOrthoWidth (Variables|Default|GetSceneCapture)) :!class /Script/Engine.KismetMaterialLibrary))

(event EventTick
  (params (DeltaSeconds :type Float%20%28single-precision%29)))

(fn ConstructionScript)

(fn DrawtoPersistent)

(fn MoveCapture)